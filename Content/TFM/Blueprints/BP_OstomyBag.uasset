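; BP_OstomyBag is a grabbable VR ostomy bag that attaches to a stoma socket on the player's avatar or a mirror avatar.
; On BeginPlay it attaches to the mirror avatar if one is set, otherwise caches the XR pawn and optionally starts attached.
; Grabbing clears the attached flag and signals removal.
; When snapping is allowed, dropping within snap distance of the avatar's bag transform reattaches it and signals the snap.
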(event `self.ReceiveBeginPlay`
  (`/Engine/EditorBlueprintResources/StandardMacros.IsValid` (`self.MirrorAvatarRef`)
    (:`Is Valid`
      (`self.AttachToMirrorStoma`))
    (:`Is Not Valid`
      (bind _asbp_xrpawn (cast `/Game/XRFramework/Blueprints/BP_XRPawn` (`GameplayStatics.GetPlayerPawn` 0)))
      (set `self.AvatarRef` _asbp_xrpawn)
      (if (`self.bStartAttached`)
        (`self.AttachToStoma`)))))

(event `self.GrabComponent.OnGrabbed`
  (`KismetSystemLibrary.PrintString` "OstomyBag Grabbed")
  (set `self.IsAttachedToStoma` false)
  (`self.OnOstomyBagRemoved`))

(event `self.GrabComponent.OnDropped`
  (if (`self.bCanSnapToStoma`)
    (bind _ostomybagtransform (`/Game/XRFramework/Blueprints/BP_XRPawn.GetOstomyBagTransform` (`self.AvatarRef`)))
    (bind _returnvalue (`KismetMathLibrary.Vector_Distance` (.location _ostomybagtransform) (`self.K2_GetActorLocation`)))
    (if (<= _returnvalue (`self.SnapDistance`))
      (`self.AttachToStoma`)
      (`KismetSystemLibrary.PrintString` "SNAPPED")
      (`self.OnBagSnappedToStoma`)
      (else
        (`KismetSystemLibrary.PrintString` (`KismetStringLibrary.Concat_StrStr` "CANT APPEND. DISTANCE: " (`KismetStringLibrary.Conv_DoubleToString` _returnvalue)))))))

(fn `AttachToMirrorStoma`
  (`self.K2_AttachToComponent` (`/Game/TFM/Blueprints/BP_MirrorAvatar.SK_NoShirt` (`self.MirrorAvatarRef`)) (`self.SocketName`) "SnapToTarget" "SnapToTarget" "KeepWorld" false)
  (set `self.IsAttachedToMirrorStoma` true))

(fn `AttachToStoma`
  (`self.K2_AttachToComponent` (`/Game/XRFramework/Blueprints/BP_XRPawn.AvatarMesh` (`self.AvatarRef`)) (`self.SocketName`) "SnapToTarget" "SnapToTarget" "KeepWorld" false)
  (set `self.IsAttachedToStoma` true))

(fn `UserConstructionScript`
  (`parent.UserConstructionScript`))