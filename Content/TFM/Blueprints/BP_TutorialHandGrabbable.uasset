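; BP_TutorialHandGrabbable is an actor, named as a tutorial hand grabbable, that can attach itself to the XR player avatar.
; On BeginPlay it casts player pawn 0 to BP_XRPawn and caches it as the avatar reference.
; Its AttachToAvatar event snaps it to a variable-named socket on the avatar's SKShirt component, keeping world scale.
; No grab logic appears in this graph, and nothing here calls the attach event.
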(event `self.ReceiveBeginPlay`
  (bind _asbp_xrpawn (cast `/Game/XRFramework/Blueprints/BP_XRPawn` (`GameplayStatics.GetPlayerPawn` 0)))
  (set `self.AvatarRef` _asbp_xrpawn))

(event `AttachToAvatar`
  (`self.K2_AttachToComponent` (`/Game/XRFramework/Blueprints/BP_XRPawn.SK_Shirt` (`self.AvatarRef`)) (`self.SocketName`) "SnapToTarget" "SnapToTarget" "KeepWorld"))

(fn `UserConstructionScript`
  (`parent.UserConstructionScript`))