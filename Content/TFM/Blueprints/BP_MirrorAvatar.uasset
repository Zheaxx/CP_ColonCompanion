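; BP_MirrorAvatar is a mirror double of the VR player's avatar, with toggleable tutorial hand meshes.
; On BeginPlay it feeds the XR pawn's avatar mesh to ABP_Mirror on its shirtless and clothed meshes.
; Tick reflects the avatar's position across world X=0 and negates its yaw.
; When the pawn's phenotype is applied, it copies morph target weights to the shirtless mesh only.
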(event `self.ReceiveBeginPlay`
  (bind _asabp_mirror (cast `/Game/Art/Mesh/ABP_Mirror` (`SkeletalMeshComponent.GetAnimInstance` (`self.SK_NoShirt`))))
  (bind _asabp_mirror_2 (cast `/Game/Art/Mesh/ABP_Mirror` (`SkeletalMeshComponent.GetAnimInstance` (`self.SK_WithClothes`))))
  (bind _asbp_xrpawn (cast `/Game/XRFramework/Blueprints/BP_XRPawn` (`GameplayStatics.GetPlayerPawn` 0)))
  (bind _avatarmesh (`/Game/XRFramework/Blueprints/BP_XRPawn.AvatarMesh` _asbp_xrpawn))
  (set `/Game/Art/Mesh/ABP_Mirror.Source Mesh Component` _avatarmesh _asabp_mirror)
  (set `/Game/Art/Mesh/ABP_Mirror.Source Mesh Component` _avatarmesh _asabp_mirror_2)
  (set `self.AvatarMeshRef` _avatarmesh)
  (add `/Game/XRFramework/Blueprints/BP_XRPawn.OnFenotypeApplied` _asbp_xrpawn (delegate `ClonePawnFenotype`)))

(event `ClonePawnFenotype`
  (`self.ClonePawnMorphTargets` (`self.AvatarMeshRef`)))

(event `ToggleFirstTutorialHand`
  (params (ShowHand :type Boolean))
  (`SceneComponent.SetHiddenInGame` (`self.SM_TutorialHand1`) (not ShowHand) false))

(event `self.ReceiveTick`
  (params (DeltaSeconds :type "Float (single-precision)"))
  (bind (_returnvalue_x _returnvalue_y) (`KismetMathLibrary.BreakVector` (`SceneComponent.K2_GetComponentLocation` (`self.AvatarMeshRef`))))
  (bind (_returnvalue_roll _returnvalue_pitch _returnvalue_yaw) (`KismetMathLibrary.BreakRotator` (`SceneComponent.K2_GetComponentRotation` (`self.AvatarMeshRef`))))
  (if (`KismetSystemLibrary.IsValid` (`self.AvatarMeshRef`))
    (`self.K2_SetActorLocation` (`KismetMathLibrary.MakeVector` (- 0.0 _returnvalue_x) _returnvalue_y))
    (`self.K2_SetActorRotation` (`KismetMathLibrary.MakeRotator` _returnvalue_roll _returnvalue_pitch (* _returnvalue_yaw -1.0)))))

(event `ToggleSecondTutorialHand`
  (params (`Show Hand` :type Boolean))
  (`SceneComponent.SetHiddenInGame` (`self.SM_TutorialHand2`) (not `Show Hand`) false))

(fn `ClonePawnMorphTargets`
  (params (PlayerAvatarSK :type "SkeletalMeshComponent Object Reference"))
  (for _array_element (`SkeletalMesh.K2_GetAllMorphTargetNames` (`SkeletalMeshComponent.GetSkeletalMeshAsset` PlayerAvatarSK))
    (bind _returnvalue (`KismetStringLibrary.Conv_StringToName` _array_element))
    (`SkeletalMeshComponent.SetMorphTarget` (`self.SK_NoShirt`) _returnvalue (`SkeletalMeshComponent.GetMorphTarget` PlayerAvatarSK _returnvalue) true)))

(fn `UserConstructionScript`)