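; BP_Avatar is an avatar actor with a skeletal mesh shaped by morph targets and a widget that shows the avatar menu.
; On construction and again at BeginPlay, InitMaleMorphTargets applies every name and weight row from the DT_MaleMorphTargetsBase data table to the mesh.
; BeginPlay first passes the mesh to WBP_AvatarMenu, and skips that morph initialization if the widget cast fails.
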(event `self.ReceiveBeginPlay`
  (bind _aswbp_avatar_menu (cast `/Game/TFM/Blueprints/UI/WBP_AvatarMenu` (`WidgetComponent.GetWidget` (`self.Widget`))))
  (set `/Game/TFM/Blueprints/UI/WBP_AvatarMenu.Avatar` (`self.SkeletalMesh`) _aswbp_avatar_menu)
  (`self.InitMaleMorphTargets`))

(event `self.ReceiveTick`
  (params (DeltaSeconds :type "Float (single-precision)")))

(fn `InitMaleMorphTargets`
  (bind _outrownames (`DataTableFunctionLibrary.GetDataTableRowNames` "/Game/TFM/Blueprints/Data/DT_MaleMorphTargetsBase.DT_MaleMorphTargetsBase"))
  (for _array_element _outrownames
    (bind _returnvalue (`|GetDataTableRow` "/Game/TFM/Blueprints/Data/DT_MaleMorphTargetsBase.DT_MaleMorphTargetsBase" _array_element)
      (:`then`
        (`SkeletalMeshComponent.SetMorphTarget` (`self.SkeletalMesh`) (break `/Game/TFM/Blueprints/Data/S_MaleMorphTargetsBase` _returnvalue) (`.Weight_5_57D9EB3B4BB57729F5D0899BBB9E7B71` (break `/Game/TFM/Blueprints/Data/S_MaleMorphTargetsBase` _returnvalue)) true)))))

(fn `UserConstructionScript`
  (`self.InitMaleMorphTargets`))